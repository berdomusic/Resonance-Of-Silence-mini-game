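; BP_SoundCharged_Crystal is the "Sound Crystal" item, handling its HUD and visual effect.
; Its HUD events swap the chargeable crystal widget into the viewport, binding it to this item, or remove it.
; EffectsSpline's VFX activation event plays or reverses a timeline that scales particle size and density, deactivating the effect once the reverse finishes.
; No charging logic appears in this Blueprint's graphs.
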(event Custom|OnVFXActivated_Event
  (params (bInResult :type Boolean))
  (bind _vfx (Variables|Default|GetVFX))
  ;[0.15 0.15 0.15 0.5] VFX
  (if bInResult
    (Components|Activation|Activate (Variables|Default|GetVFX) false)
    (bind (_direction _size) (Timeline|VFX%20sze Play)
      (:Update
        (Effects|Components|ParticleSystem|SetFloatParameter _vfx "_Size" _size)
        (Effects|Components|ParticleSystem|SetFloatParameter _vfx "Count(Density)" (* _size 1e+01)))
      (:Finished
        (switch Utilities|FlowControl|Switch|SwitchonETimelineDirection _direction
          (:Backward
            (Components|Activation|Deactivate _vfx)))))
    (else
      (Timeline|VFX%20sze Reverse))))

(event EventAddItemHUD
  (params (InItem :type RS%20Pickable%20Item%20Object%20Reference))
  ;[0.15 0.15 0.15 0.5] HUD
  (Class|RSUISubsystem|SwapWidgetinViewport (Subsystems|GetRSUISubsystem) (Variables|Default|GetItemHUDWidget))
  (bind _aswbp_chargable_sound_crystal (Utilities|Casting|CastToWBP_ChargableSoundCrystal (Variables|Default|GetItemHUDWidget)))
  (Variables|/Game/UI/Widgets/Items/WBP_ChargableSoundCrystal.WBP_ChargableSoundCrystal_C|SetOwner _aswbp_chargable_sound_crystal self)
  (Default|BindEvents _aswbp_chargable_sound_crystal))

(event EventRemoveItemHUD
  (params (InItem :type RS%20Pickable%20Item%20Object%20Reference))
  ;[0.15 0.15 0.15 0.5] HUD
  (Class|RSUISubsystem|RemoveWidgetfromViewport (Subsystems|GetRSUISubsystem) (Variables|Default|GetItemHUDWidget)))

(event EventBeginPlay
  ;[0.15 0.15 0.15 0.5] VFX
  (EventDispatchers|AssignOnVFXActivated (Variables|Default|GetEffectsSpline) (delegate Custom|OnVFXActivated_Event)))

(fn ConstructionScript)

(fn GetItemName
  (return "Sound Crystal"))