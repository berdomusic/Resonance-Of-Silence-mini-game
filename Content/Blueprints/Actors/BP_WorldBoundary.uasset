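; BP_WorldBoundary is a spline-based world boundary actor that provides visual feedback for the boundary and for players being pushed back.
; ManageSplineVFX toggles the boundary VFX and, on activation, starts async loading the push-back effect.
; OnPlayerPushedBack spawns that soft-referenced effect at the supplied transform; the push itself is not in these graphs.
; The construction script snaps CollisionSphere to the spline's first point.
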(event EventManageSplineVFX
  (params (bInActive :type Boolean))
  (bind _vfx (Variables|Default|GetVFX))
  (if bInActive
    (Components|Activation|Activate _vfx false)
    (Utilities|AsyncLoadAsset (Variables|Default|GetPushBackVFX))
    (else
      (Components|Activation|Deactivate _vfx))))

(event EventOnPlayerPushedBack
  (params (InTrans :type Transform))
  (Niagara|SpawnSystematLocation (Utilities|ResolveSoftReference (Variables|Default|GetPushBackVFX)) (.location InTrans) (.rotation InTrans)))

(fn ConstructionScript
  (Transformation|SetWorldLocation (Variables|Default|GetCollisionSphere) (Spline|GetLocationatSplinePoint (Variables|Default|GetBoundarySpline) 0 "World") false false))