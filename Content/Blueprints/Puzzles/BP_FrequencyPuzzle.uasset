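; Frequency puzzle actor that gates a path with sliding doors, a blocking box, a completion light and an optional rotating bridge.
; It registers with RSPuzzleSubsystem, then on activation async-loads soft-referenced crystals and a prize item to bind pickup and drop events.
; Charging ramps the bobbing spheres' timeline play rate through a second timeline, sized by the difficulty's charging time.
; Received sound rotates the bridge, and debug text shows the required frequency range.
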(event Custom|RotateBridge
  (params (bIsAccessible :type Boolean))
  (bind _bridgeroty (Variables|Default|GetBridgeRotY))
  (bind _bridge (Variables|Default|GetBridge))
  (bind _relativerotation (Variables|/Script/Engine.SceneComponent|GetRelativeRotation _bridge))
  ;[0.15 0.15 0.15 0.5] Bridge
  (if (Variables|Default|GetbHasBridge)
    (if bIsAccessible
      (if (not (.bwassolved (Variables|Default|GetCurrentPuzzleState)))
        (bind _alpha (Timeline|BridgeRot Reverse)
          (:Update
            (Transformation|SetRelativeRotation (Variables|Default|GetBridge) (Math|Rotator|MakeRotator (.roll _relativerotation) (Math|Float|Lerp _bridgeroty (+ _bridgeroty 9e+01) _alpha) (.yaw _relativerotation)) false false))))
      (else
        (Timeline|BridgeRot Play)))))

(event Custom|ChangeLights
  (params (bUnlock :type Boolean))
  (bind _completionlight (Variables|Default|GetCompletionLight))
  ;[0.15 0.15 0.15 0.5] CompletionLight
  (if bUnlock
    (Rendering|Components|Light|SetLightColor _completionlight "(R=0.000000,G=1.000000,B=0.024677,A=1.000000)" true)
    (elif (not (.bwassolved (Variables|Default|GetCurrentPuzzleState)))
      (Rendering|Components|Light|SetLightColor _completionlight "(R=1.000000,G=0.002493,B=0.000000,A=1.000000)" true))))

(event Custom|DEBUG_OnDifficultyChange
  (params (InNewDifficulty :type ERSGameDifficulty%20Enum :default "Easy"))
  ;[0.15 0.15 0.15 0.5] DEBUG
  ;;[0.15 0.15 0.15 0.5] wait for update
  (Utilities|FlowControl|DelayUntilNextTick)
  (Development|PrintString (Utilities|String|Append "DEBUG: 
New Difficulty is " (Utilities|String|EnumtoString InNewDifficulty) " 
Sound charging time is " (Utilities|String|ToString(Float) (.ChargingTime (Utilities|Struct|BreakRSFrequencyPuzzleDifficulty (Variables|Default|GetCurrentPuzzleDifficulty))))) true true "(R=0.000000,G=0.660000,B=1.000000,A=1.000000)" 5.0))

(event Custom|DEBUG_ChangeHelperTextVisibility
  (params (InPuzzleHelperState :type ERSPuzzleHelper%20Enum :default "Disabled"))
  (bind _returnvalue (Utilities|Select :Index InPuzzleHelperState :Disabled false :Enabled true))
  ;[0.15 0.15 0.15 0.5] DEBUG
  (Rendering|SetVisibility (Variables|Default|GetHelperText) _returnvalue false)
  (Rendering|SetVisibility (Variables|Default|GetCrystalActivationText) _returnvalue false)
  (Rendering|SetVisibility (Variables|Default|GetCrystalChargingText) _returnvalue false))

(event EventBeginPlay
  (bind _chargingupsphere (Variables|Default|GetChargingUpSphere))
  (bind _crystalactivationsphere (Variables|Default|GetCrystalActivationSphere))
  (bind _relativelocation (Variables|/Script/Engine.SceneComponent|GetRelativeLocation _chargingupsphere))
  (bind _relativelocation_2 (Variables|/Script/Engine.SceneComponent|GetRelativeLocation _crystalactivationsphere))
  ;[0.15 0.15 0.15 0.5] Begin/End play
  (Class|RSPuzzleSubsystem|ActivatePuzzle (Subsystems|GetRSPuzzleSubsystem) self)
  (Utilities|FlowControl|Sequence
    (:then_0
      (bind _alpha (Timeline|ChargeUpSphereMovement PlayFromStart)
        (:Update
          (Transformation|SetRelativeLocation _chargingupsphere (Math|Vector|MakeVector (.x _relativelocation) (.y _relativelocation) (+ _alpha (Variables|Default|GetChargeUpSphereInitZ))) false false)
          (Transformation|SetRelativeLocation _crystalactivationsphere (Math|Vector|MakeVector (.x _relativelocation_2) (.y _relativelocation_2) (- (Variables|Default|GetCrystalActivationSphereInit) _alpha)) false false))))
    (:then_1
      ;;[0.15 0.15 0.15 0.5] DEBUG
      (EventDispatchers|BindEventtoOnDifficultyChanged (Class|RSGameUserSettings|Get) (EventDispatchers|CreateEvent :!event Custom|DEBUG_OnDifficultyChange))
      (EventDispatchers|BindEventtoOnPuzzleHelperStateChange (Class|RSCheatManager|GetCheatManager) (EventDispatchers|CreateEvent :!event Custom|DEBUG_ChangeHelperTextVisibility)))
    (:then_2
      (CallFunction|DEBUGChangeHelperTextVisibility (Class|RSCheatManager|GetPuzzleHelper)))))

(event EventOpenDoors
  (bind _door1initx (Variables|Default|GetDoor1InitX))
  ;[0.15 0.15 0.15 0.5] Doors
  (if (.bwassolved (Variables|Default|GetCurrentPuzzleState))
    (bind (_direction _alpha) (Timeline|DoorOpening Play)
      (:Update
        (Transformation|SetRelativeLocation (Variables|Default|GetDoor1) (Math|Vector|MakeVector (Math|Float|Lerp _door1initx (+ _door1initx -1.5e+02) _alpha) 0.0 0.0) false false)
        (Transformation|SetRelativeLocation (Variables|Default|GetDoor2) (Math|Vector|MakeVector (Math|Float|Lerp (Variables|Default|GetDoor2InitX) (+ (Variables|Default|GetDoor2InitX) 1.5e+02) _alpha) 0.0 0.0) false false))
      (:Finished
        (switch Utilities|FlowControl|Switch|SwitchonETimelineDirection _direction
          (:Forward
            (Class|RSPuzzleBase|ChangeBlockersAccessibility true (Utilities|Array|MakeArray (Variables|Default|GetBlockingBox)))
            (CallFunction|ChangeLights true)))))
    (else
      (CallFunction|RotateBridge false)
      (Timeline|DoorOpening Play))))

(event EventOnSolvingConditionUpdate
  ;[0.15 0.15 0.15 0.5] Difficulty change
  (Components|Timeline|SetTimelineLength (Variables|Default|GetChargeUpSphereMovementInterp) (Utilities|Struct|BreakRSFrequencyPuzzleDifficulty (Variables|Default|GetCurrentPuzzleDifficulty)))
  (CallFunction|UpdateHelperText))

(event EventOnReceivedTransmittedSound
  (params (InData :type RS%20Transmitted%20Sound%20Data%20Structure%20%28by%20ref%29))
  ;[0.15 0.15 0.15 0.5] Receiving sound
  (|CallParentFunction InData)
  (CallFunction|RotateBridge true))

(event EventCloseDoors
  (bind _door1initx (Variables|Default|GetDoor1InitX))
  ;[0.15 0.15 0.15 0.5] Doors
  (if (not (.bwassolved (Variables|Default|GetCurrentPuzzleState)))
    (CallFunction|RotateBridge true)
    (Class|RSPuzzleBase|ChangeBlockersAccessibility false (Utilities|Array|MakeArray (Variables|Default|GetBlockingBox)))
    (CallFunction|ChangeLights false)
    (bind (_direction _alpha) (Timeline|DoorOpening Reverse)
      (:Update
        (Transformation|SetRelativeLocation (Variables|Default|GetDoor1) (Math|Vector|MakeVector (Math|Float|Lerp _door1initx (+ _door1initx -1.5e+02) _alpha) 0.0 0.0) false false)
        (Transformation|SetRelativeLocation (Variables|Default|GetDoor2) (Math|Vector|MakeVector (Math|Float|Lerp (Variables|Default|GetDoor2InitX) (+ (Variables|Default|GetDoor2InitX) 1.5e+02) _alpha) 0.0 0.0) false false))
      (:Finished
        (switch Utilities|FlowControl|Switch|SwitchonETimelineDirection _direction
          (:Forward
            (Class|RSPuzzleBase|ChangeBlockersAccessibility true (Utilities|Array|MakeArray (Variables|Default|GetBlockingBox)))
            (CallFunction|ChangeLights true)))))))

(event EventActivatePuzzle
  (bind _associatedcrystalssoft (Variables|Default|GetAssociatedCrystalsSoft))
  (bind _prizeitemsoft (Variables|Default|GetPrizeItemSoft))
  ;[0.15 0.15 0.15 0.5] Activation
  (|CallParentFunction)
  (|LoadSoftArrayAsync _associatedcrystalssoft
    (:OnSoftArrayLoaded
      (for _array_element _associatedcrystalssoft
        (CallFunction|BindEvents (Utilities|ResolveSoftReference _array_element)))
      (Utilities|AsyncLoadAsset _prizeitemsoft
        (:Completed
          (EventDispatchers|BindEventtoOnItemPickedUp (Utilities|ResolveSoftReference _prizeitemsoft) (EventDispatchers|CreateEvent :!event OnPrizeCollected)))))))

(event EventStartCharging
  ;[0.15 0.15 0.15 0.5] Charging
  (|CallParentFunction)
  (bind _newrate (Timeline|ChargeUpSphereMovementInterp Play)
    (:Update
      (Components|Timeline|SetPlayRate (Variables|Default|GetChargeUpSphereMovement) _newrate))))

(event EventStopCharging
  ;[0.15 0.15 0.15 0.5] Charging
  (|CallParentFunction)
  (bind _newrate (Timeline|ChargeUpSphereMovementInterp Reverse)
    (:Update
      (Components|Timeline|SetPlayRate (Variables|Default|GetChargeUpSphereMovement) _newrate))))

(event EventEndPlay
  (params (EndPlayReason :type EEndPlayReason%20Enum :default "Destroyed"))
  ;[0.15 0.15 0.15 0.5] Begin/End play
  (Class|RSPuzzleSubsystem|DeactivatePuzzle (Subsystems|GetRSPuzzleSubsystem) self))

(event EventDeactivatePuzzle
  ;[0.15 0.15 0.15 0.5] Activation
  (|CallParentFunction))

(fn ConstructionScript
  (bind _doorscale (Variables|Default|GetDoorScale))
  (bind _blockingbox (Variables|Default|GetBlockingBox))
  (bind _doorscale_2 (Variables|Default|GetDoorScale))
  (bind _returnvalue (* _doorscale 5e+01))
  (bind _boxextent (Variables|/Script/Engine.BoxComponent|GetBoxExtent _blockingbox))
  (bind _returnvalue_2 (Math|Vector|MakeVector _returnvalue 0.0 0.0))
  (Utilities|FlowControl|Sequence
    (:then_0
      (for _array_element (Utilities|Array|MakeArray (Variables|Default|GetDoor1) (Variables|Default|GetDoor2))
        (Transformation|SetWorldScale3D _array_element (Math|Conversions|ToVector(Float) (Variables|Default|GetDoorScale))))
      (Transformation|SetRelativeLocation (Variables|Default|GetDoor1) (* _returnvalue_2 "-1.000000,0.000000,0.000000") false false)
      (Transformation|SetRelativeLocation (Variables|Default|GetDoor2) _returnvalue_2 false false)
      (Components|Box|SetBoxExtent _blockingbox (Math|Vector|MakeVector (* (.x _boxextent) _doorscale_2) 1.0 (* (.z _boxextent) _doorscale_2)) false))
    (:then_1
      (Variables|Default|SetDoor1InitX (.x (Variables|/Script/Engine.SceneComponent|GetRelativeLocation (Variables|Default|GetDoor1))))
      (Variables|Default|SetDoor2InitX (.x (Variables|/Script/Engine.SceneComponent|GetRelativeLocation (Variables|Default|GetDoor2))))
      (Variables|Default|SetChargeUpSphereInitZ (.z (Variables|/Script/Engine.SceneComponent|GetRelativeLocation (Variables|Default|GetChargingUpSphere))))
      (Variables|Default|SetCrystalActivationSphereInit (+ (.z (Variables|/Script/Engine.SceneComponent|GetRelativeLocation (Variables|Default|GetCrystalActivationSphere))) 25.0))
      (Variables|Default|SetBridgeRotY (.pitch (Transformation|GetWorldRotation (Variables|Default|GetBridge)))))
    (:then_2
      (bind _output_get (Variables|Default|SetbHasBridge (Variables|/Script/Engine.SceneComponent|GetbVisible (Variables|Default|GetBridge))))
      (Collision|SetCollisionProfileName (Variables|Default|GetBridge) (Utilities|String|SelectName "BlockDynamicNoCamera" "NoCollision" _output_get) false :!class /Script/Engine.PrimitiveComponent))
    (:then_3
      (CallFunction|UpdateHelperText))))

(fn BindEvents
  (params (InCrystal :type RS%20Sound%20Charged%20Crystal%20Object%20Reference))
  (EventDispatchers|BindEventtoOnItemPickedUp InCrystal (EventDispatchers|CreateEvent :!event OnChargingCrystalPickup))
  (EventDispatchers|BindEventtoOnItemDroppedStart InCrystal (EventDispatchers|CreateEvent :!event OnChargingCrystalDropped)))

(fn UpdateHelperText
  (bind _helpertext (Variables|Default|GetHelperText))
  (bind _currentsolvingcondition (Variables|Default|GetCurrentSolvingCondition))
  (bind _currentpuzzledifficulty (Variables|Default|GetCurrentPuzzleDifficulty))
  (bind _matchingfrequencytolerance (Utilities|Struct|BreakRSFrequencyPuzzleDifficulty _currentpuzzledifficulty))
  (Rendering|Components|TextRender|SetText _helpertext (Utilities|Text|ToText(String) (Utilities|String|Append "Current solving frequency is in range: " (Utilities|String|ToString(Integer) (- (.requiredfrequency _currentsolvingcondition) _matchingfrequencytolerance)) " Hz to " (Utilities|String|ToString(Integer) (+ (.requiredfrequency _currentsolvingcondition) _matchingfrequencytolerance)) " Hz")))
  (Rendering|SetVisibility _helpertext (Utilities|Select :Index (Class|RSCheatManager|GetPuzzleHelper) :Disabled false :Enabled true) false))